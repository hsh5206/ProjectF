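; Game instance that wraps online session create, find and join for non-LAN play, printing each outcome to screen.
; Creating a session opens 127.0.0.1 on success; joining uses the search result stored on the main menu player controller.
; Both then switch to game-only input and hide the cursor.
; Finding sessions only checks the first result's index, without acting on it.
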(event Custom|Create%20Session
  (params (PublicConnections :type Integer))
  (bind _returnvalue (Game|GetPlayerController 0))
  (|Session (Game|GetPlayerController 0) PublicConnections false
    (:OnSuccess
      (Development|PrintString "Create Session!")
      (Game|OpenLevel(byName) "127.0.0.1")
      (Input|SetInputModeGameOnly _returnvalue false)
      (Variables|/Script/Engine.PlayerController|SetbShowMouseCursor _returnvalue false))
    (:OnFailure
      (Development|PrintString "Failed to Create Session" true true "(R=1.000000,G=0.000000,B=0.000000,A=1.000000)"))))

(event Custom|Find%20Sessions
  (bind _results (|FindSessions (Game|GetPlayerController 0) 20 false)
    (:OnSuccess
      (Development|PrintString "Find Session!")
      (if (Utilities|Array|IsValidIndex _results)
        _))
    (:OnFailure
      (Development|PrintString "Failed to Find Session" true true "(R=1.000000,G=0.000000,B=0.000000,A=1.000000)"))))

(event Custom|Join%20Session
  (bind _returnvalue (Game|GetPlayerController 0))
  (bind _asbp_player_controller_main_menu (Utilities|Casting|CastToBP_PlayerController_MainMenu (Game|GetPlayerController 0)))
  (|JoinSession _asbp_player_controller_main_menu (Variables|/Game/Blueprints/Frameworks/MainMenu/BP_PlayerController_MainMenu.BP_PlayerController_MainMenu_C|GetWantToJoinSessionResult _asbp_player_controller_main_menu)
    (:OnSuccess
      (Development|PrintString "Join Session!")
      (Input|SetInputModeGameOnly _returnvalue false)
      (Variables|/Script/Engine.PlayerController|SetbShowMouseCursor _returnvalue false))
    (:OnFailure
      (Development|PrintString "Failed to Join Session" true true "(R=1.000000,G=0.000000,B=0.000000,A=1.000000)"))))